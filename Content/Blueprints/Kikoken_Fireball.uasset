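; Kikoken fireball projectile, likely Chun-Li's, that knocks back a Dummy_Blueprint on hit and gets a movement push along X at BeginPlay.
; Tick chains up to three debug-drawn line traces on the facing side as a hitbox, playing a sound and launching the dummy on contact.
; It writes DummyHit to GameInstance_Demo, then destroys itself on a hit or otherwise refreshes its flipbook and facing from ChunFacesRight.
; Overlap and Hit events are empty.
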(event `self.ReceiveActorBeginOverlap`
  (params (OtherActor :type "Actor Object Reference"))
  ;[1 1 1] (Old) Handle Collision
)

(event `self.ReceiveHit`
  (params (MyComp :type "PrimitiveComponent Object Reference") (Other :type "Actor Object Reference") (OtherComp :type "PrimitiveComponent Object Reference") (bSelfMoved :type Boolean) (HitLocation :type "Vector Structure") (HitNormal :type "Vector Structure") (NormalImpulse :type "Vector Structure") (Hit :type "HitResult Structure (by ref)"))
  ;[1 1 1] (Old) Handle Collision
)

(event `self.ReceiveBeginPlay`
  ;[1 1 1] (Old) Handle Walking
  (if (`self.facesRight`)
    (`self.AddMovementInput` (1.0 0.0 0.0) 1.0 true)
    (else
      (`self.AddMovementInput` (-1.0 0.0 0.0) 1.0 true))))

(event `Update Animation`
  ;[1 1 1] Handle Animation
  (`PaperFlipbookComponent.SetFlipbook` (`self.Sprite`) (select `bool` (`self.facesRight`) :`false` "/Game/2DSideScroller/Sprites/Chun-Li/Special_Moves/Fireball_Kikoken/Fireball_Kikoken_Flipbook.Fireball_Kikoken_Flipbook" :`true` "/Game/2DSideScroller/Sprites/Chun-Li/Special_Moves/Fireball_Kikoken/Fireball_Kikoken_Flipbook.Fireball_Kikoken_Flipbook" :!type "PaperFlipbook Object Reference")))

(event `self.ReceiveTick`
  (params (DeltaSeconds :type "Float (single-precision)"))
  ;[1 1 1] Tick - Updates animation
  ;[1 1 1] Working Handle Collision
  (bind _output_get (set `self.Fireball Location` (`self.K2_GetActorLocation`)))
  (if (`self.facesRight`)
    (bind _returnvalue (+ _output_get (0.0 0.0 -10.0)))
    (bind (_outhit _returnvalue_2) (`KismetSystemLibrary.LineTraceSingleForObjects` :`Start` _returnvalue :`End` (+ _returnvalue (10.0 0.0 30.0)) :`ObjectTypes` (`self.Object Types`) :`DrawDebugType` "ForDuration" :`DrawTime` (`self.fireballActive`)))
    (if _returnvalue_2
      (bind (_bblockinghit _binitialoverlap _time _distance _location _impactpoint _normal _impactnormal _physmat _hitactor _hitcomponent _hitbonename _hititem _faceindex _tracestart _traceend) (`GameplayStatics.BreakHitResult` _outhit))
      (set `self.Hit Actor` _hitactor)
      (`GameplayStatics.PlaySound2D` "/Game/2DSideScroller/Sounds/SE_00033.SE_00033" 1.0 1.0 0.0 null null :!label _label)
      (bind _asdummy_blueprint (cast `/Game/Blueprints/Dummy_Blueprint` (`self.Hit Actor`)))
      (`self.LaunchCharacter` _asdummy_blueprint (300.0 0.0 0.0) true true)
      (else
        (bind (_outhit_2 _returnvalue_3) (`KismetSystemLibrary.LineTraceSingleForObjects` :`Start` _traceend :`End` (+ _traceend (0.0 0.0 -10.0)) :`ObjectTypes` (`self.Object Types`) :`DrawDebugType` "ForDuration" :`DrawTime` (`self.fireballActive`)))
        (if _returnvalue_3
          (bind (_bblockinghit_2 _binitialoverlap_2 _time_2 _distance_2 _location_2 _impactpoint_2 _normal_2 _impactnormal_2 _physmat_2 _hitactor_2 _hitcomponent_2 _hitbonename_2 _hititem_2 _faceindex_2 _tracestart_2 _traceend_2) (`GameplayStatics.BreakHitResult` _outhit_2))
          (set `self.Hit Actor` _hitactor_2)
          (goto _label)
          (else
            (bind (_outhit_3 _returnvalue_4) (`KismetSystemLibrary.LineTraceSingleForObjects` :`Start` _traceend_2 :`End` (+ _traceend_2 (20.0 0.0 0.0)) :`ObjectTypes` (`self.Object Types`) :`DrawDebugType` "ForDuration" :`DrawTime` (`self.fireballActive`)))
            (if _returnvalue_4
              (set `self.Hit Actor` (`.HitActor` (`GameplayStatics.BreakHitResult` _outhit_3)))
              (goto _label)
              (else
                _))))))
    (else
      (bind _returnvalue_5 (+ _output_get (0.0 0.0 -10.0)))
      (bind (_outhit_4 _returnvalue_6) (`KismetSystemLibrary.LineTraceSingleForObjects` :`Start` _returnvalue_5 :`End` (+ _returnvalue_5 (-10.0 0.0 30.0)) :`ObjectTypes` (`self.Object Types`) :`DrawDebugType` "ForDuration" :`DrawTime` (`self.fireballActive`)))
      (if _returnvalue_6
        (bind (_bblockinghit_3 _binitialoverlap_3 _time_3 _distance_3 _location_3 _impactpoint_3 _normal_3 _impactnormal_3 _physmat_3 _hitactor_3 _hitcomponent_3 _hitbonename_3 _hititem_3 _faceindex_3 _tracestart_3 _traceend_3) (`GameplayStatics.BreakHitResult` _outhit_4))
        (set `self.Hit Actor` _hitactor_3)
        (`GameplayStatics.PlaySound2D` "/Game/2DSideScroller/Sounds/SE_00033.SE_00033" 1.0 1.0 0.0 null null :!label _label_2)
        (bind _asdummy_blueprint_2 (cast `/Game/Blueprints/Dummy_Blueprint` (`self.Hit Actor`)))
        (`self.LaunchCharacter` _asdummy_blueprint_2 (-300.0 0.0 0.0) true true)
        (else
          (bind (_outhit_5 _returnvalue_7) (`KismetSystemLibrary.LineTraceSingleForObjects` :`Start` _traceend_3 :`End` (+ _traceend_3 (0.0 0.0 10.0)) :`ObjectTypes` (`self.Object Types`) :`DrawDebugType` "ForDuration" :`DrawTime` (`self.fireballActive`)))
          (if _returnvalue_7
            (bind (_bblockinghit_4 _binitialoverlap_4 _time_4 _distance_4 _location_4 _impactpoint_4 _normal_4 _impactnormal_4 _physmat_4 _hitactor_4 _hitcomponent_4 _hitbonename_4 _hititem_4 _faceindex_4 _tracestart_4 _traceend_4) (`GameplayStatics.BreakHitResult` _outhit_5))
            (set `self.Hit Actor` _hitactor_4)
            (goto _label_2)
            (else
              (bind (_outhit_6 _returnvalue_8) (`KismetSystemLibrary.LineTraceSingleForObjects` :`Start` _traceend_4 :`End` (+ _traceend_4 (-20.0 0.0 0.0)) :`ObjectTypes` (`self.Object Types`) :`DrawDebugType` "ForDuration" :`DrawTime` (`self.fireballActive`)))
              (if _returnvalue_8
                (set `self.Hit Actor` (`.HitActor` (`GameplayStatics.BreakHitResult` _outhit_6)))
                (goto _label_2)
                (else
                  _))))))))
  (bind _asgame_instance_demo (cast `/Game/Blueprints/GameInstance_Demo` (`GameplayStatics.GetGameInstance`)))
  (bind _output_get_2 (set `/Game/Blueprints/GameInstance_Demo.dummyHit` (or _returnvalue_4 _returnvalue_3 _returnvalue_2 _returnvalue_8 _returnvalue_7 _returnvalue_6) _asgame_instance_demo))
  (if _output_get_2
    (`KismetSystemLibrary.PrintString` "it hit!!!!!!!!!!!")
    (`self.K2_DestroyActor`)
    (else
      (`self.Update Animation`)
      (bind _asgame_instance_demo_2 (cast `/Game/Blueprints/GameInstance_Demo` (`GameplayStatics.GetGameInstance`)))
      (if (`/Game/Blueprints/GameInstance_Demo.chunFacesRight` _asgame_instance_demo_2)
        (set `self.facesRight` true)
        (`self.K2_SetActorRotation` (`KismetMathLibrary.MakeRotator` 0.0))
        (else
          (set `self.facesRight` false)
          (`self.K2_SetActorRotation` (`KismetMathLibrary.MakeRotator` 0.0 0.0 180.0)))))))

(fn `Fierce Detected`)

(fn `UserConstructionScript`)